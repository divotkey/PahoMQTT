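; BP_MQTT_Sender is an example actor that periodically publishes MQTT messages through an MQTT plugin.
; On BeginPlay it binds to the MQTT Subsystem's connected delegate, then starts a looping timer at MessageInterval once connected.
; Each SendMessage call uses the elapsed game time as payload, prints it and publishes it to Topic via the Blueprint Library, a convenience wrapper around the subsystem.
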(event Custom|Connection%20Established
  ;[1 1 1] We bind a custom event to the `OnMQTTConnected` delegate from the MQTT Subsystem.
  ; This ensures we do not publish messages without a valid connection
  (Utilities|Time|SetTimerbyFunctionName 0 "SendMessage" (Variables|Default|GetMessage%20Interval) true))

(event EventBeginPlay
  ;[1 1 1] We bind a custom event to the `OnMQTTConnected` delegate from the MQTT Subsystem.
  ; This ensures we do not publish messages without a valid connection
  (EventDispatchers|BindEventtoOnMQTTConnected (Subsystems|GetMQTTSubsystem) (delegate Custom|Connection%20Established)))

(event Collision|EventActorBeginOverlap
  (params (OtherActor :type Actor%20Object%20Reference)))

(event EventTick
  (params (DeltaSeconds :type Float%20%28single-precision%29)))

(fn ConstructionScript)

(fn SendMessage
  (Utilities|FlowControl|Sequence
    (:then_0
      ;[1 1 1] Assemble message payload
      ; IN this example we use the elapsed game time.
      (LocalVariables|SetPayload (Utilities|String|ToString(Float) (Utilities|Time|GetGameTimeinSeconds))))
    (:then_1
      ;[1 1 1] Emit some Debug/Log Messages
      (Development|PrintString (Utilities|String|Append "Sending MQTT Message: '" (LocalVariables|GetPayload))))
    (:then_2
      ;[1 1 1] Publish the MQTT Message using the Blueprint Library function.
      (Class|MQTTBlueprintLibrary|PublishMessage (Variables|Default|GetTopic) (LocalVariables|GetPayload) 1 false))))