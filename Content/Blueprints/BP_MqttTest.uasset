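; Test actor that exercises a Simple MQTT client against a hardcoded local broker.
; On BeginPlay it constructs and initializes the client, binds connection and message callbacks, then connects.
; On connect it logs success and subscribes to temperature and debug test topics.
; Each received message is printed to screen and answered by publishing a fixed reply to a separate test topic.
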(event Custom|OnConnected
  (bind _client (Variables|Default|GetClient))
  (Utilities|String|LogString "Successfully connected to MQTT Broker")
  (Class|SimpleMQTTClient|SubscribeTopic _client "test/temperature" 0)
  (Class|SimpleMQTTClient|SubscribeTopic _client "test/debug" 0))

(event Custom|OnMessage
  (params (Topic :type String) (Message :type String))
  (Development|PrintString (Utilities|String|Append "MQTT Message: " Topic " - " Message))
  (Class|SimpleMQTTClient|PublishMessage (Variables|Default|GetClient) "test/unreal" "Unreal likes MQTT" 0 false))

(event EventBeginPlay
  (Utilities|FlowControl|Sequence
    (:then_0
      (bind _returnvalue (Game|ConstructObjectfromClass "/Script/PahoMQTT.SimpleMQTTClient"))
      (bind _output_get (Variables|Default|SetClient _returnvalue))
      (Class|SimpleMQTTClient|InitializeClient _output_get "mqtt://192.168.0.24:1883" "UnrealClient"))
    (:then_1
      (EventDispatchers|BindEventtoOnConnected (Variables|Default|GetClient) (delegate Custom|OnConnected))
      (EventDispatchers|BindEventtoOnMessageReceived (Variables|Default|GetClient) (delegate Custom|OnMessage))
      (Class|SimpleMQTTClient|Connect (Variables|Default|GetClient)))))

(event Collision|EventActorBeginOverlap
  (params (OtherActor :type Actor%20Object%20Reference)))

(event EventTick
  (params (DeltaSeconds :type Float%20%28single-precision%29)))

(fn ConstructionScript)