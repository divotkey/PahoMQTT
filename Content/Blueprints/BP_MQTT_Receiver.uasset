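; Example MQTT receiver actor that subscribes to the "sensor/updates" topic and displays incoming messages.
; On BeginPlay it binds to the MQTT Subsystem's connected and message-received delegates, deferring the QoS 1 subscription until the broker connection is established.
; HandleMessage counts messages and updates the count, topic and payload texts, while each message is also printed for debugging.
; Topic filtering is skipped because only one topic is subscribed.
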(event Custom|Connection%20Established
  ;[1 1 1] We bind a custom event to the `OnMQTTConnected` delegate from the MQTT Subsystem.
  ;
  ; This ensures we only subscribe to a topic after the connection to the broker is established.
  (Rendering|Components|TextRender|SetText (Variables|Default|GetConnected) (Variables|Default|GetConntectedText))
  (Development|PrintString "Successfully connected to MQTT Broker")
  (Class|MQTTBlueprintLibrary|SubscribetoTopic "sensor/updates" 1))

(event Custom|New%20MQTT%20Message
  (params (Topic :type String) (Message :type String))
  ;[1 1 1] Bind to the OnMQTTMessageReceived event to react to incoming MQTT messages.
  ;
  ; Since we are only subscribed to a single topic in this example, we skip checking the topic name.
  ; The received payload is simply printed to the screen for demonstration purposes.
  (CallFunction|HandleMessage Topic Message)
  (Development|PrintString (Utilities|String|Append "MQTT Message - Topic: \"" Topic "\" - Payload \"" Message "\"")))

(event EventBeginPlay
  (Utilities|FlowControl|Sequence
    (:then_0
      ;[1 1 1] We bind a custom event to the `OnMQTTConnected` delegate from the MQTT Subsystem.
      ;
      ; This ensures we only subscribe to a topic after the connection to the broker is established.
      (EventDispatchers|BindEventtoOnMQTTConnected (Subsystems|GetMQTTSubsystem) (delegate Custom|Connection%20Established)))
    (:then_1
      ;[1 1 1] Bind to the OnMQTTMessageReceived event to react to incoming MQTT messages.
      ;
      ; Since we are only subscribed to a single topic in this example, we skip checking the topic name.
      ; The received payload is simply printed to the screen for demonstration purposes.
      (EventDispatchers|BindEventtoOnMQTTMessageReceived (Subsystems|GetMQTTSubsystem) (delegate Custom|New%20MQTT%20Message)))))

(event Collision|EventActorBeginOverlap
  (params (OtherActor :type Actor%20Object%20Reference)))

(event EventTick
  (params (DeltaSeconds :type Float%20%28single-precision%29)))

(fn ConstructionScript)

(fn HandleMessage
  (params (Topic :type String) (Message :type String))
  (Utilities|FlowControl|Sequence
    (:then_0
      ;[1 1 1] Update Message Counter
      (bind _result (Math|Integer|IncrementInt (Variables|Default|GetNumMessages))
        (:%20%20
          (Rendering|Components|TextRender|SetText (Variables|Default|GetMessage%20Count) (Utilities|Text|ToText(String) (Utilities|String|Append "Received Messages: " (Utilities|String|ToString(Integer) _result)))))))
    (:then_1
      ;[1 1 1] Update Topic Text
      (Rendering|Components|TextRender|SetText (Variables|Default|GetTopic) (Utilities|Text|ToText(String) (Utilities|String|Append "Topic: " Topic))))
    (:then_2
      ;[1 1 1] Update Message Text
      (Rendering|Components|TextRender|SetText (Variables|Default|GetPayload) (Utilities|Text|ToText(String) (Utilities|String|Append "Message Payload: " Message))))))